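; Game mode for a target-shooting style game that tracks score against the number of BP_Target actors in the level.
; On BeginPlay it counts the targets as MaxScore, then creates WBP_UI, adds it to the viewport and refreshes it.
; AddScore increments CurrentScore, updates the widget, and prints a win message once the score equals MaxScore.
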(event Custom|Add%20Score
  (bind _result (Math|Integer|IncrementInt (Variables|Default|GetCurrentScore))
    (:%20%20
      (Variables|Default|SetCurrentScore _result)
      (Default|UpdateScore (Variables|Default|GetUIRef))
      (if (== (Variables|Default|GetCurrentScore) (Variables|Default|GetMaxScore))
        (Development|PrintString "Won!!" true true "(R=1.000000,G=0.000000,B=0.028078,A=1.000000)" 1e+02)))))

(event EventBeginPlay
  (Utilities|FlowControl|Sequence
    (:then_0
      (bind _outactors (Actor|GetAllActorsOfClass "/Game/GameEx/Blueprints/BP_Target.BP_Target_C"))
      (Variables|Default|SetMaxScore (Utilities|Array|Length _outactors)))
    (:then_1
      (bind _returnvalue (UserInterface|CreateWidget "/Game/GameEx/UI/WBP_UI.WBP_UI_C"))
      (bind _output_get (Variables|Default|SetUIRef _returnvalue))
      (UserInterface|Viewport|AddtoViewport _output_get 0)
      (Default|UpdateScore _output_get))))

(event EventTick
  (params (DeltaSeconds :type Float%20%28single-precision%29)))

(fn ConstructionScript)